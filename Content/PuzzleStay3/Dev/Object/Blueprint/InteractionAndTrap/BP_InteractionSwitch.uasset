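; BP_InteractionSwitch is an interactable switch object that shows an interaction prompt to nearby players.
; Box overlap events filter for a PS3PlayerCharacter, then call ShowInteractionUI on InteractionSwitch to show the prompt on entry and hide it on exit.
; A locally controlled check limits the prompt to the overlapping player's own client.
; The graph holds no switch activation logic, and the construction script is empty.
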(event OnComponentBeginOverlap(Box)
  (params (OverlappedComponent :type Primitive%20Component%20Object%20Reference) (OtherActor :type Actor%20Object%20Reference) (OtherComp :type Primitive%20Component%20Object%20Reference) (OtherBodyIndex :type Integer) (bFromSweep :type Boolean) (SweepResult :type Hit%20Result%20Structure%20%28by%20ref%29))
  (bind _asps3player_character (Utilities|Casting|CastToPS3PlayerCharacter OtherActor))
  (if (Pawn|IsLocallyControlled _asps3player_character)
    (Class|InteractionSwitchComponent|ShowInteractionUI (Variables|Default|GetInteractionSwitch) true)))

(event OnComponentEndOverlap(Box)
  (params (OverlappedComponent :type Primitive%20Component%20Object%20Reference) (OtherActor :type Actor%20Object%20Reference) (OtherComp :type Primitive%20Component%20Object%20Reference) (OtherBodyIndex :type Integer))
  (bind _asps3player_character (Utilities|Casting|CastToPS3PlayerCharacter OtherActor))
  (if (Pawn|IsLocallyControlled _asps3player_character)
    (Class|InteractionSwitchComponent|ShowInteractionUI (Variables|Default|GetInteractionSwitch) false)))

(fn ConstructionScript)