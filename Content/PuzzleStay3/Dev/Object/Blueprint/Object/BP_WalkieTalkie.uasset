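; BP_WalkieTalkie is an interactable walkie-talkie pickup that changes a player's voice chat state when picked up.
; CanInteract accepts any PS3PlayerCharacter while nobody holds it.
; On the server, Interact acquires the voice object through the controller's CustomVoiceComponent, sets the PlayerState to Conversion and attaches the actor to a mesh socket.
; The replicated HoldingPlayer's OnRep disables physics and collision, matching what the server does on pickup.
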(event EventBeginPlay)

(event Collision|EventActorBeginOverlap
  (params (OtherActor :type Actor%20Object%20Reference)))

(event EventTick
  (params (DeltaSeconds :type Float%20%28single-precision%29)))

(fn ConstructionScript)

(fn OnRepHoldingPlayer
  (Utilities|IsValid (Variables|Default|GetHoldingPlayer)
    (:Is%20Valid
      (Physics|SetSimulatePhysics (Variables|Default|GetStaticMesh) false)
      (Collision|SetActorEnableCollision false))))

(fn CanInteract
  (params (Requestor :type Actor%20Object%20Reference))
  (if (Utilities|IsValid (Variables|Default|GetHoldingPlayer))
    (return false)
    (else
      (Utilities|Casting|CastToPS3PlayerCharacter Requestor
        (:then
          (return true))
        (:CastFailed
          (return false))))))

(fn Interact
  (params (Requestor :type Actor%20Object%20Reference))
  (Networking|SwitchHasAuthority
    (:Authority
      (if (Utilities|IsValid (Variables|Default|GetHoldingPlayer))
        (return false)
        (else
          (bind _asps3player_character (Utilities|Casting|CastToPS3PlayerCharacter Requestor)
            (:then
              (Utilities|IsValid (Actor|GetComponentbyClass (Pawn|GetController _asps3player_character) "/Script/PuzzleStay3.CustomVoiceComponent")
                (:Is%20Valid
                  (bind _asps3player_state (Utilities|Casting|CastToPS3PlayerState (Variables|/Script/Engine.Pawn|GetPlayerState _asps3player_character))
                    (:then
                      (bind _returnvalue (Class|CustomVoiceComponent|TryAcquireVoiceObject (Actor|GetComponentbyClass (Pawn|GetController _asps3player_character) "/Script/PuzzleStay3.CustomVoiceComponent")))
                      (if _returnvalue
                        (Class|PS3PlayerState|SetVoiceChatState _asps3player_state "Conversion")
                        (Variables|Default|SetHoldingPlayer _asps3player_character)
                        (Physics|SetSimulatePhysics (Variables|Default|GetStaticMesh) false)
                        (Collision|SetActorEnableCollision false)
                        (Transformation|AttachComponentToComponent (Variables|/Script/Engine.Character|GetMesh (Variables|Default|GetHoldingPlayer)) "WalkieTalkieSocket" "SnapToTarget" "SnapToTarget" "KeepWorld" false)
                        (return true)
                        (else
                          (return false))))
                    (:CastFailed
                      (return false))))))
            (:CastFailed
              (return false))))))
    (:Remote
      (return false))))