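; BP_EOSLobbyTestController is a player controller for testing the EOS lobby through an on-screen widget.
; On BeginPlay, only for the local controller, it creates WBP_EOSLobby_Test and adds it to the viewport.
; It then switches input to Game and UI focused on that widget and shows the mouse cursor.
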(event EventBeginPlay
  (|CallParentFunction)
  (if (Pawn|IsLocalController)
    (bind _returnvalue (UserInterface|CreateWidget "/Game/PuzzleStay3/Dev/UI/Widget/WBP_EOSLobby_Test.WBP_EOSLobby_Test_C" self))
    (UserInterface|Viewport|AddtoViewport _returnvalue 0)
    (Input|SetInputModeGameandUI self _returnvalue "DoNotLock" true false)
    (Variables|Default|SetbShowMouseCursor true)))

(fn ConstructionScript
  (|CallParentFunction))