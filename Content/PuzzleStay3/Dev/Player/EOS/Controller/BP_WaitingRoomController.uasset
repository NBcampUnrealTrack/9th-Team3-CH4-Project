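; BP_WaitingRoomController is the player controller for the waiting room that precedes a two-player match.
; On BeginPlay, the local controller shows the WBP_WaitingRoom widget, enables the mouse cursor and switches input to Game and UI.
; TryStartGame acts only on the local controller with authority, and when exactly two players are present it runs a one-time ServerTravel console command to TestStage1.
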(event Custom|TryStartGame
  (if (Pawn|IsLocalController)
    (Networking|SwitchHasAuthority
      (:Authority
        (if (== (Utilities|Array|Length (Variables|/Script/Engine.GameStateBase|GetPlayerArray (Game|GetGameState))) 2)
          (Utilities|FlowControl|DoOnce false
            (:Completed
              (Development|ExecuteConsoleCommand "ServerTravel /Game/PuzzleStay3/Dev/Maps/TestStage1" 0))))))))

(event EventBeginPlay
  (if (Pawn|IsLocalController)
    (bind _returnvalue (UserInterface|CreateWidget "/Game/PuzzleStay3/Dev/UI/Widget/WBP_WaitingRoom.WBP_WaitingRoom_C"))
    (UserInterface|Viewport|AddtoViewport _returnvalue 0)
    (Variables|Default|SetbShowMouseCursor true)
    (Input|SetInputModeGameandUI self 0 "DoNotLock" true false)))

(fn ConstructionScript)