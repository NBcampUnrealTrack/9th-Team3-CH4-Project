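; Player character Blueprint for PuzzleStay3 that gives each player a distinct body based on player identity.
; The ApplyPlayerIdentityVisual event swaps the skeletal mesh to the Mario model for Player 1 or the Luigi model for Player 2.
; BeginPlay waits briefly, then prints the role from the PS3PlayerState as debug output, independently of the mesh swap.
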(event EventBeginPlay
  (Utilities|FlowControl|Delay 1.0)
  (bind _asps3player_state (Utilities|Casting|CastToPS3PlayerState (Game|GetPlayerState 0)))
  (Development|PrintString (Utilities|String|EnumtoString (Class|PS3PlayerState|GetPlayerRole _asps3player_state))))

(event EventApplyPlayerIdentityVisual
  (params (PlayerIdentity :type EPS3PlayerIdentity%20Enum :default "Unassigned"))
  (switch Utilities|FlowControl|Switch|SwitchonEPS3PlayerIdentity PlayerIdentity
    (:Player1
      (Components|SkeletalMesh|SetSkeletalMeshAsset (Variables|Character|GetMesh) "/Game/PuzzleStay3/Dev/Asset/PS3_PlayerCharacterMesh/Meshes/SK_Mario_Character.SK_Mario_Character"))
    (:Player2
      (Components|SkeletalMesh|SetSkeletalMeshAsset (Variables|Character|GetMesh) "/Game/PuzzleStay3/Dev/Asset/PS3_PlayerCharacterMesh/Meshes/SK_Luige_Character.SK_Luige_Character"))))

(fn ConstructionScript)